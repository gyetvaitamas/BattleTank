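; Tank Blueprint that handles player camera aiming through horizontal and vertical input axes.
; AimHorizontal yaws VerticalGimbal and AimVertical pitches the SpringArm, splitting the two rotations across separate components.
; Both apply local rotation scaled by AimSpeed and world delta time for frame-rate independence, with no pitch clamp in the graph.
; The event graph and construction script hold no logic.
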(event `InputAxis|AimHorizontal`
  (params (AxisValue :type "Float (single-precision)"))
  ;[1 1 1] Camera input binding
  ;;[1 1 1] X-axis aiming
  (`SceneComponent.K2_AddLocalRotation` (`self.VerticalGimbal`) (`KismetMathLibrary.MakeRotator` 0.0 0.0 (* AxisValue (`GameplayStatics.GetWorldDeltaSeconds`) (`self.AimSpeed`))) false false))

(event `InputAxis|AimVertical`
  (params (AxisValue :type "Float (single-precision)"))
  ;[1 1 1] Camera input binding
  ;;[1 1 1] Y-axis aiming
  (`SceneComponent.K2_AddLocalRotation` (`self.SpringArm`) (`KismetMathLibrary.MakeRotator` 0.0 (* AxisValue (`GameplayStatics.GetWorldDeltaSeconds`) (`self.AimSpeed`))) false false))

(fn `UserConstructionScript`)